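; BP_EliteUnit is an RTS unit that relays move and stop orders to its AI controller's Blackboard.
; On possession it caches the AIC_EliteUnit controller.
; Move and stop events set TargetLocation, but write a separate MoveToLocation variable, never assigned in these graphs, to the MoveToLocation key.
; AttackTarget is a placeholder that only prints a debug string.
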(event EventAttackTarget
  (params (target :type Object%20Object%20Reference))
  (Development|PrintString "Shoot"))

(event EventPossessed
  (params (NewController :type Controller%20Object%20Reference))
  (bind _asaic_elite_unit (Utilities|Casting|CastToAIC_EliteUnit NewController))
  (Variables|Default|SetAIController _asaic_elite_unit))

(event EventSetMoveLocation
  (params (targetLocation :type Vector :default "0, 0, 0"))
  (Variables|Default|SetTarget%20Location targetLocation)
  (AI|Components|Blackboard|SetValueasVector (AI|GetBlackboard (Variables|Default|GetAIController)) (Utilities|Name|MakeLiteralName "MoveToLocation") (Variables|Default|GetMoveToLocation)))

(event EventStopMoving
  (Variables|Default|SetTarget%20Location (Transformation|GetActorLocation))
  (AI|Components|Blackboard|SetValueasVector (AI|GetBlackboard (Variables|Default|GetAIController)) (Utilities|Name|MakeLiteralName "MoveToLocation") (Variables|Default|GetMoveToLocation)))

(fn ConstructionScript)